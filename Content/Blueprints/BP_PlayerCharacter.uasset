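; Player character Blueprint that uses Enhanced Input for single-axis movement and a prototype hold-to-interact action.
; BeginPlay adds the movement mapping context, and IA_Movement drives movement input along world Y.
; IA_Interact compares elapsed hold time to HoldValue, which the InteractionTime event sets.
; Interaction only prints debug text so far, and the hold-complete message sits behind a DoOnce with no visible reset.
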(event `self.ReceiveBeginPlay`
  (bind _asbp_player_controller (cast `/Game/Blueprints/BP_PlayerController` (`self.GetController`)))
  (`EnhancedInputSubsystemInterface.AddMappingContext` (pcsubsystem `EnhancedInputLocalPlayerSubsystem` _asbp_player_controller) "/Game/Blueprints/IMC_playerCharacterMovement.IMC_playerCharacterMovement" 0 (struct)))

(event `EnhancedInput|/Game/Blueprints/IA_Movement`
  (params (ActionValue :type "Float (double-precision)") (ElapsedSeconds :type "Float (double-precision)") (TriggeredSeconds :type "Float (double-precision)") (InputAction :type "InputAction Object Reference" :default "/Game/Blueprints/IA_Movement.IA_Movement"))
  (:`Triggered`
    (`self.AddMovementInput` (0.0 1.0 0.0) ActionValue)))

(event `EnhancedInput|/Game/Blueprints/IA_Interact`
  (params (ActionValue :type "Float (double-precision)") (ElapsedSeconds :type "Float (double-precision)") (TriggeredSeconds :type "Float (double-precision)") (InputAction :type "InputAction Object Reference" :default "/Game/Blueprints/IA_Interact.IA_Interact"))
  (bind _returnvalue (`KismetStringLibrary.Conv_DoubleToString` ElapsedSeconds))
  (:`Started`
    (`KismetSystemLibrary.PrintString` "Hello"))
  (:`Ongoing`
    (if (>= ElapsedSeconds (`self.Hold Value`))
      (`/Engine/EditorBlueprintResources/StandardMacros.DoOnce` false
        (:`Completed`
          (`KismetSystemLibrary.PrintString` (`KismetStringLibrary.Concat_StrStr` "HOLD " _returnvalue))))
      (else
        (`KismetSystemLibrary.PrintString` (`KismetStringLibrary.Concat_StrStr` "wait" _returnvalue))))))

(event `/Game/Blueprints/boxes/BPI_interactionTime.InteractionTime`
  (params (InteractionTime :type "Float (double-precision)"))
  (bind _output_get (set `self.Hold Value` InteractionTime))
  (`KismetSystemLibrary.PrintString` (`KismetStringLibrary.Concat_StrStr` "HOLD VALUE: " (`KismetStringLibrary.Conv_DoubleToString` _output_get))))

(fn `UserConstructionScript`)